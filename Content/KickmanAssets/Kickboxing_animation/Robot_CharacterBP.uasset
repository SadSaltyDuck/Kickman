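; Modular robot kickboxing character, player-controlled or not, with a montage kick on left click that halts movement and has a cooldown.
; Another character overlapping BodyCapsule knocks the robot away, damages it and briefly stuns it.
; Timed checks while falling escalate damage applied on landing.
; At zero health, body parts detach from the master pose to simulate physics, movement and capsule collision stop, and ABP_Robot is flagged dead.
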(event OnComponentBeginOverlap(BodyCapsule)
  (params (OverlappedComponent :type Primitive%20Component%20Object%20Reference) (OtherActor :type Actor%20Object%20Reference) (OtherComp :type Primitive%20Component%20Object%20Reference) (OtherBodyIndex :type Integer) (bFromSweep :type Boolean) (SweepResult :type Hit%20Result%20Structure%20%28by%20ref%29))
  ;[1 1 1] Collision physics
  (if (!= OtherActor self)
    (bind _ascharacter (Utilities|Casting|CastToCharacter OtherActor))
    (Animation|StopAnimMontage 0)
    (Pawn|Components|CharacterMovement|SetMovementMode (Variables|Character|GetCharacterMovement) "MOVE_Walking" 0)
    (Character|LaunchCharacter (Math|Vector|MakeVector (.X (Math|Vector|BreakVector (* (Math|Vector|GetUnitDirection(Vector) (Transformation|GetActorLocation _ascharacter) (Transformation|GetActorLocation)) "2000.000000,2000.000000,1.000000"))) (.Y (Math|Vector|BreakVector (* (Math|Vector|GetUnitDirection(Vector) (Transformation|GetActorLocation _ascharacter) (Transformation|GetActorLocation)) "2000.000000,2000.000000,1.000000"))) (.Z (Math|Vector|BreakVector (* (Math|Vector|GetUnitDirection(Vector) (Transformation|GetActorLocation _ascharacter) (Transformation|GetActorLocation)) "2000.000000,2000.000000,1.000000")))) false false)
    (Game|Damage|ApplyDamage self 4e+01 0 0)
    (Utilities|FlowControl|Delay 0.3)
    (Pawn|Components|CharacterMovement|SetMovementMode (Variables|Character|GetCharacterMovement) "MOVE_None" 0)
    (Utilities|FlowControl|Delay 0.4)
    (Pawn|Components|CharacterMovement|SetMovementMode (Variables|Character|GetCharacterMovement) "MOVE_Walking" 0)
    (else
      (Development|PrintString "Stop Hitting Yourself "))))

(event Custom|KickEvent
  ;[1 1 1] Kicking with cooldown
  (if (and (not (AI|Components|NavMovement|IsFalling (Pawn|GetMovementComponent))) (Variables|Default|GetCanKick))
    (Animation|Montage|PlayMontage (Variables|Character|GetMesh) "/Game/KickmanAssets/Kickboxing_animation/Animations/Kick_Montage.Kick_Montage"
      (:then
        (Pawn|Components|CharacterMovement|SetMovementMode (Variables|Character|GetCharacterMovement) "MOVE_None" 0)
        (Variables|Default|SetCanKick false)
        (Utilities|FlowControl|Delay 3.0)
        (Variables|Default|SetCanKick true))
      (:OnCompleted
        (Pawn|Components|CharacterMovement|SetMovementMode (Variables|Character|GetCharacterMovement) "MOVE_Walking" 0)))))

(event Game|Damage|EventAnyDamage
  (params (Damage :type Float%20%28single-precision%29) (DamageType :type Damage%20Type%20Object%20Reference) (InstigatedBy :type Controller%20Object%20Reference) (DamageCauser :type Actor%20Object%20Reference))
  (bind _returnvalue (Utilities|String|MakeLiteralString "health left"))
  ;[1 1 1] Damage and physics
  (Variables|Default|SetHealth (- (Variables|Default|GetHealth) Damage))
  (if (> (Variables|Default|GetHealth) 0.0)
    (if (Pawn|IsPlayerControlled self)
      (Development|PrintString (Utilities|String|Append (Utilities|String|MakeLiteralString "I have ") (Utilities|String|ToString(Float) (Variables|Default|GetHealth)) _returnvalue))
      (else
        (Development|PrintString (Utilities|String|Append (Utilities|String|MakeLiteralString "Robot has") (Utilities|String|ToString(Float) (Variables|Default|GetHealth)) _returnvalue))))
    (else
      (Class|SkinnedMeshComponent|SetMasterPoseComponent (Variables|Default|GetRightLeg) 0 true)
      (Physics|SetSimulatePhysics (Variables|Character|GetMesh) true)
      (Pawn|Components|CharacterMovement|DisableMovement (Variables|Character|GetCharacterMovement))
      (bind _asabp_robot (Utilities|Casting|CastToABP_Robot (Components|SkeletalMesh|GetAnimInstance (Variables|Character|GetMesh))))
      (Variables|/Game/KickmanAssets/Kickboxing_animation/Animations/ABP_Robot.ABP_Robot_C|SetIsAlive _asabp_robot false)
      (Collision|SetCollisionEnabled (Variables|Collision|GetCapsuleComponent) "NoCollision"))))

(event EventOnMovementModeChanged
  (params (PrevMovementMode :type EMovementMode%20Enum :default "MOVE_None") (NewMovementMode :type EMovementMode%20Enum :default "MOVE_None") (PrevCustomMode :type Byte :default 0) (NewCustomMode :type Byte :default 0))
  (bind _charactermovement (Variables|Character|GetCharacterMovement))
  (bind _returnvalue (AI|Components|NavMovement|IsFalling _charactermovement))
  (if (Utilities|Enum|Equal(Enum) NewMovementMode "MOVE_Falling")
    (Utilities|FlowControl|RetriggerableDelay 1.0)
    (if _returnvalue
      (Variables|Default|SetTemporaryDamage 4e+01)
      (Utilities|FlowControl|RetriggerableDelay 0.25)
      (if _returnvalue
        (Variables|Default|SetTemporaryDamage 8e+01)
        (Utilities|FlowControl|RetriggerableDelay 0.25)
        (if _returnvalue
          (Variables|Default|SetTemporaryDamage 1e+02))))))

(event EventOnLanded
  (params (Hit :type Hit%20Result%20Structure%20%28by%20ref%29))
  (Game|Damage|ApplyDamage self (Variables|Default|GetTemporaryDamage) 0 0)
  (Variables|Default|SetTemporaryDamage 0.0))

(event Input|MouseEvents|LeftMouseButton
  (params (Key :type Key%20Structure :default "None"))
  ;[1 1 1] Kicking with cooldown
  (:Pressed
    (CallFunction|KickEvent)))

(fn ConstructionScript
  (Class|SkinnedMeshComponent|SetMasterPoseComponent (Variables|Default|GetRightLeg) (Variables|Character|GetMesh) false))

(fn UpdateWalkSpeed
  (params (New%20Walk%20Speed :type Float%20%28double-precision%29))
  (Variables|/Script/Engine.CharacterMovementComponent|SetMaxWalkSpeed (Variables|Character|GetCharacterMovement) New%20Walk%20Speed))